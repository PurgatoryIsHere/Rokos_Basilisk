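; Enemy spawner that scatters basic melee or ranged AI across the navmesh around itself at BeginPlay.
; The spawn count follows EnemyDensity from BP_BasiliskInstance, with a roughly even random pick between BP_Basic_AI and BP_Basic_AI_Ranged.
; Each position comes from two chained random navigable-point lookups with a random X offset between them.
; Points too far above the first-person character drop to that character's height.
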(event EventBeginPlay
  (bind _asbp_basilisk_instance (Utilities|Casting|CastToBP_BasiliskInstance (Game|GetGameInstance)))
  (for _index (range 0 (Math|Float|Truncate (- (Variables|/Game/BP_BasiliskInstance.BP_BasiliskInstance_C|GetEnemyDensity _asbp_basilisk_instance) 1.0)))
    (bind _randomlocation (Class|NavigationSystemV1|GetRandomLocationinNavigableRadius (Transformation|GetActorLocation) 1e+04 0 0))
    (bind _randomlocation_2 (Class|NavigationSystemV1|GetRandomLocationinNavigableRadius (+ _randomlocation (Math|Vector|MakeVector (Math|Random|RandomFloatinRange 0.0 1e+04) 0.0 1e+02)) 1e+03 0 0))
    (bind _returnvalue (Actor|GetActorOfClass "/Game/FirstPerson/Blueprints/BP_FirstPersonCharacter.BP_FirstPersonCharacter_C"))
    (if (> (.z _randomlocation_2) (+ (.z (Transformation|GetActorLocation _returnvalue)) 1e+02))
      (if (<= (Math|Random|RandomFloatinRange 0.0 1e+01) 5.0)
        (Game|SpawnActorfromClass "/Game/Enemies/EnemyAI/BP_Basic_AI.BP_Basic_AI_C" (Math|Transform|MakeTransform (Math|Vector|MakeVector (.x _randomlocation_2) (.y _randomlocation_2) (.z (Transformation|GetActorLocation _returnvalue))) "0, 0, 0" "1.000000,1.000000,1.000000") "AdjustIfPossibleButDontSpawnIfColliding" "MultiplyWithRoot" 0 0)
        (else
          (Game|SpawnActorfromClass "/Game/Enemies/RangedEnemy/BP_Basic_AI_Ranged.BP_Basic_AI_Ranged_C" (Math|Transform|MakeTransform (Math|Vector|MakeVector (.x _randomlocation_2) (.y _randomlocation_2) (.z (Transformation|GetActorLocation _returnvalue))) "0, 0, 0" "1.000000,1.000000,1.000000") "AdjustIfPossibleButDontSpawnIfColliding" "MultiplyWithRoot" 0 0)))
      (elif (<= (Math|Random|RandomFloatinRange 0.0 1e+01) 5.0)
        (Game|SpawnActorfromClass "/Game/Enemies/EnemyAI/BP_Basic_AI.BP_Basic_AI_C" (Math|Transform|MakeTransform (Math|Vector|MakeVector (.x _randomlocation_2) (.y _randomlocation_2) (.z _randomlocation_2)) "0, 0, 0" "1.000000,1.000000,1.000000") "AdjustIfPossibleButDontSpawnIfColliding" "MultiplyWithRoot" 0 0)
        (else
          (Game|SpawnActorfromClass "/Game/Enemies/RangedEnemy/BP_Basic_AI_Ranged.BP_Basic_AI_Ranged_C" (Math|Transform|MakeTransform (Math|Vector|MakeVector (.x _randomlocation_2) (.y _randomlocation_2) (.z _randomlocation_2)) "0, 0, 0" "1.000000,1.000000,1.000000") "AdjustIfPossibleButDontSpawnIfColliding" "MultiplyWithRoot" 0 0))))))

(fn ConstructionScript)