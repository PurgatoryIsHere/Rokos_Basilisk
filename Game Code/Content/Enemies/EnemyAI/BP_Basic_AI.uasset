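; Base melee enemy character that scales to the game instance's difficulty, takes damage and reports its death to the game mode.
; Attack plays a montage whose notify fires a forward sphere trace against pawns to apply damage.
; At zero health it passes location and survival time to the game mode, switches the capsule to overlap and expires shortly after.
; Tick destroys it in the height-based kill field, decrementing EnemiesAlive directly.
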(event EventAttack
  (bind _returnvalue (Transformation|GetActorLocation))
  (if (not false)
    (Animation|Montage|PlayMontage (Variables|Character|GetMesh) "/Game/Characters/Mannequins/Animations/Melee_Attack.Melee_Attack"
      (:OnNotifyBegin
        (bind (_outhit _returnvalue_2) (Collision|SphereTraceForObjects _returnvalue (+ _returnvalue (* (Math|Vector|GetForwardVector (Transformation|GetActorRotation)) 1.7e+02)) 3e+01 (Utilities|Array|MakeArray "ObjectTypeQuery3") false 0 "None"))
        (if _returnvalue_2
          (bind _returnvalue_3 (Class|CBasicAI|GetDamageDealt))
          (Game|Damage|ApplyDamage (.HitActor (Collision|BreakHitResult _outhit)) _returnvalue_3 0 0))))))

(event EventTick
  (params (DeltaSeconds :type Float%20%28single-precision%29))
  (bind _returnvalue (Class|CBasicAI|KillField (.z (Transformation|GetActorLocation))))
  (if _returnvalue
    (Class|CBasicAI|GetTimeSurvived)
    (Actor|DestroyActor)
    (bind _returnvalue_2 (Actor|GetActorOfClass "/Game/FirstPerson/Blueprints/BP_FirstPersonGameMode.BP_FirstPersonGameMode_C"))
    (Variables|/Game/FirstPerson/Blueprints/BP_FirstPersonGameMode.BP_FirstPersonGameMode_C|SetEnemiesAlive _returnvalue_2 (- (Variables|/Game/FirstPerson/Blueprints/BP_FirstPersonGameMode.BP_FirstPersonGameMode_C|GetEnemiesAlive _returnvalue_2) 1))))

(event EventBeginPlay
  (bind _asbp_basilisk_instance (Utilities|Casting|CastToBP_BasiliskInstance (Game|GetGameInstance)))
  (Class|CBasicAI|AdjustDifficultySettings (Variables|/Game/BP_BasiliskInstance.BP_BasiliskInstance_C|GetDifficulty _asbp_basilisk_instance)))

(event Game|Damage|EventAnyDamage
  (params (Damage :type Float%20%28single-precision%29) (DamageType :type Damage%20Type%20Object%20Reference) (InstigatedBy :type Controller%20Object%20Reference) (DamageCauser :type Actor%20Object%20Reference))
  (Class|CBasicAI|TakeDamage Damage)
  (if (== (Variables|Default|GetHealth) 0.0)
    (bind _returnvalue (Class|CBasicAI|GetTimeSurvived))
    (bind _asbp_first_person_game_mode (Utilities|Casting|CastToBP_FirstPersonGameMode (Game|GetGameMode)))
    (Default|EnemyDeath _asbp_first_person_game_mode (Transformation|GetActorLocation) _returnvalue)
    (Collision|SetCollisionResponsetoAllChannels (Variables|Default|GetCapsuleComponent) "ECR_Overlap")
    (Actor|SetLifeSpan 3.0)))

(fn ConstructionScript)