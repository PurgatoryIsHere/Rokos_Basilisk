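; BP_Basic_AI_Controller is the AI controller for basic enemies, running the BT_Basic_AI behavior tree on BeginPlay.
; Its AI Perception updates filter for actors tagged "Player" and set the "isSeeingPlayer" Blackboard bool to whether the stimulus was successfully sensed.
; The same result is passed to UpdateIsDetected on the BP_FirstPersonCharacter found through GetActorOfClass, so the player character tracks its detection state.
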(event OnTargetPerceptionUpdated(AIPerception)
  (params (Actor :type Actor%20Object%20Reference) (Stimulus :type AI%20Stimulus%20Structure))
  (if (Actor|ActorHasTag Actor "Player")
    (if (.bSuccessfullySensed (Utilities|Struct|BreakAIStimulus Stimulus))
      (AI|Components|Blackboard|SetValueasBool (AI|GetBlackboard 0) (Utilities|Name|MakeLiteralName "isSeeingPlayer") true)
      (bind _returnvalue (Actor|GetActorOfClass "/Game/FirstPerson/Blueprints/BP_FirstPersonCharacter.BP_FirstPersonCharacter_C"))
      (Class|CFirstPersonCharacter|UpdateIsDetected _returnvalue true)
      (else
        (AI|Components|Blackboard|SetValueasBool (AI|GetBlackboard 0) (Utilities|Name|MakeLiteralName "isSeeingPlayer") false)
        (bind _returnvalue_2 (Actor|GetActorOfClass "/Game/FirstPerson/Blueprints/BP_FirstPersonCharacter.BP_FirstPersonCharacter_C"))
        (Class|CFirstPersonCharacter|UpdateIsDetected _returnvalue_2 false)))))

(event EventBeginPlay
  (AI|RunBehaviorTree "/Game/Enemies/EnemyAI/BT_Basic_AI.BT_Basic_AI"))

(fn ConstructionScript)