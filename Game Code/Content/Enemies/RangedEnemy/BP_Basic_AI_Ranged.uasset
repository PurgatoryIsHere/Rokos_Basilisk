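; Ranged enemy that turns to face the player and plays a shoot montage, spawning a projectile on its notify, gated by a short cooldown.
; At zero health it reports death to the game mode, switches to overlap collision, expires after a delay and may drop a health pickup.
; Tick updates player distance and runs a height-based kill check that destroys it and directly decrements EnemiesAlive.
; A melee sphere-trace attack remains unconnected.
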(event EventTick
  (params (DeltaSeconds :type Float%20%28single-precision%29))
  (bind _returnvalue (Actor|GetActorOfClass "/Game/FirstPerson/Blueprints/BP_FirstPersonCharacter.BP_FirstPersonCharacter_C"))
  (Variables|Default|SetdistToPlayer (Transformation|GetDistanceTo _returnvalue))
  (bind _returnvalue_2 (Class|CBasicAI|KillField (.z (Transformation|GetActorLocation))))
  (if _returnvalue_2
    (Class|CBasicAI|GetTimeSurvived)
    (Actor|DestroyActor)
    (bind _returnvalue_3 (Actor|GetActorOfClass "/Game/FirstPerson/Blueprints/BP_FirstPersonGameMode.BP_FirstPersonGameMode_C"))
    (Variables|/Game/FirstPerson/Blueprints/BP_FirstPersonGameMode.BP_FirstPersonGameMode_C|SetEnemiesAlive _returnvalue_3 (- (Variables|/Game/FirstPerson/Blueprints/BP_FirstPersonGameMode.BP_FirstPersonGameMode_C|GetEnemiesAlive _returnvalue_3) 1))))

(event Game|Damage|EventAnyDamage
  (params (Damage :type Float%20%28single-precision%29) (DamageType :type Damage%20Type%20Object%20Reference) (InstigatedBy :type Controller%20Object%20Reference) (DamageCauser :type Actor%20Object%20Reference))
  (Class|CBasicAI|TakeDamage Damage)
  (if (== (Variables|Default|GetHealth) 0.0)
    (bind _returnvalue (Class|CBasicAI|GetTimeSurvived))
    (bind _asbp_first_person_game_mode (Utilities|Casting|CastToBP_FirstPersonGameMode (Game|GetGameMode)))
    (Default|EnemyDeath _asbp_first_person_game_mode (Transformation|GetActorLocation) _returnvalue)
    (Collision|SetCollisionResponsetoAllChannels (Variables|Default|GetCapsuleComponent) "ECR_Overlap")
    (Actor|SetLifeSpan 3.0)
    (if (<= (Math|Random|RandomInteger 100) (Variables|Default|GetHealthDropChance))
      (Game|SpawnActorfromClass "/Game/Fab/Health_potion/HealthPickup.HealthPickup_C" (Transformation|GetActorTransform) "AdjustIfPossibleButAlwaysSpawn" "MultiplyWithRoot" 0 0))))

(event EventBeginPlay)

(event Collision|EventActorBeginOverlap
  (params (OtherActor :type Actor%20Object%20Reference)))

(event EventAttackRanged
  (if (Variables|Default|GetcanAttack)
    (bind _returnvalue (Actor|GetActorOfClass "/Game/FirstPerson/Blueprints/BP_FirstPersonCharacter.BP_FirstPersonCharacter_C"))
    (Transformation|SetActorRotation (Math|Rotator|FindLookatRotation (Transformation|GetActorLocation) (Transformation|GetActorLocation _returnvalue)) true)
    (Animation|Montage|PlayMontage (Variables|Character|GetMesh) "/Game/Enemies/RangedEnemy/AnimationStuff/AnimShoot.AnimShoot"
      (:then
        (Variables|Default|SetcanAttack false)
        (Utilities|FlowControl|Delay 0.3)
        (Variables|Default|SetcanAttack true))
      (:OnNotifyBegin
        (Game|SpawnActorfromClass "/Game/Enemies/RangedEnemy/Projectile/BP_Enemy_Projectile.BP_Enemy_Projectile_C" (Transformation|GetWorldTransform (Variables|Default|GetSpawnLocation)) "Undefined" "MultiplyWithRoot" 0 0)))))

(fn ConstructionScript
  (|CallParentFunction))